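; King NPC Blueprint that places itself on a chess board square when play begins.
; BeginPlay calls SnapActorToSquare on BoardRef with its File, Rank and ZOffset, first finding a ChessBoard actor in the level if the reference is invalid.
; When the reference is already valid, it also prints debug text and, after a short delay, its resulting location.
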(event `self.ReceiveBeginPlay`
  (if (`KismetSystemLibrary.IsValid` (`self.BoardRef`))
    (`KismetSystemLibrary.PrintString` "Hello")
    (`ChessBoard.SnapActorToSquare` :`self` (`self.BoardRef`) :`ActorToSnap` self :`File` (`self.File`) :`Rank` (`self.Rank`) :`ZOffset` (`self.ZOffset`))
    (`KismetSystemLibrary.Delay` 0.5)
    (`KismetSystemLibrary.PrintString` (`KismetStringLibrary.Conv_VectorToString` (`self.K2_GetActorLocation`)))
    (else
      (bind _returnvalue (`GameplayStatics.GetActorOfClass` "/Script/ChessKids.ChessBoard"))
      (bind _output_get (set `self.BoardRef` _returnvalue))
      (`ChessBoard.SnapActorToSquare` :`self` _output_get :`ActorToSnap` self :`File` (`self.File`) :`Rank` (`self.Rank`) :`ZOffset` (`self.ZOffset`)))))

(fn `UserConstructionScript`)